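; BP_AI_Character is an NPC character that patrols a looping list of destination actors when its State is set to the matching enum value at BeginPlay.
; MoveToPoint uses AI MoveTo, advances the Target index with wraparound on success, waits a random few seconds, then calls itself again.
; A failed move has no handler, so the loop stops.
; The construction script makes the eye and brow meshes follow SyntyMesh through leader pose.
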(event Custom|MoveToPoint
  ;[0.15 0.15 0.15 0.5] Move To Point
  (AI|AIMoveTo self "0, 0, 0" (Utilities|Array|Get(acopy) (Variables|Default|GetDestinations) (Variables|Default|GetTarget)) 5.0 true
    (:OnSuccess
      (if (== (+ (Variables|Default|GetTarget) 1) (Utilities|Array|Length (Variables|Default|GetDestinations)))
        (Variables|Default|SetTarget 0)
        (else
          (Variables|Default|SetTarget (+ (Variables|Default|GetTarget) 1))))
      (Utilities|FlowControl|Delay (Math|Random|RandomFloatinRange 3.0 8.0))
      (CallFunction|MovetoPoint))))

(event EventBeginPlay
  (if (Utilities|Enum|Equal(Enum) (Variables|Default|GetState) "NewEnumerator1")
    (CallFunction|MovetoPoint)))

(fn ConstructionScript
  (Components|SkinnedMesh|SetLeaderPoseComponent (Variables|Default|GetSkeletalMesh_Eyes) (Variables|Default|GetSynty%20Mesh) false false)
  (|CallParentFunction))